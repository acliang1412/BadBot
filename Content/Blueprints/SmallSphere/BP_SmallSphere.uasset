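; BP_SmallSphere is a short-lived moving collectible that raises the BP_BadBotGameMode score when a Pawn overlaps it.
; BeginPlay scales it in via timeline, picks a random spin and starts a lifetime timer.
; Tick moves it along its forward vector while rotating the whole actor, so its heading keeps changing.
; Pickup or timeout triggers a guarded WinkOut timeline that scales the mesh, then destroys the actor.
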(event Custom|WinkOut
  ;[0.15 0.02105 0.02736 0.5] Start WinkOut TimeLine
  (if (not (Variables|Default|GetIsWinking))
    (Variables|Default|SetIsWinking true)
    (bind _scale (Timeline|WinkOutTimeLine Play)
      (:Update
        (CallFunction|ScaleSphere _scale))
      (:Finished
        (Actor|DestroyActor)))))

(event Custom|WinkIn
  ;[0.15 0.15 0.15 0.5] Wink into Existence
  (bind _scale (Timeline|Wink%20In%20Timeline Play)
    (:Update
      (Transformation|SetWorldScale3D (Variables|Default|GetSphereMesh) _scale))))

(event Custom|OnSphereOverlap
  (params (OverlappedComponent :type Primitive%20Component%20Object%20Reference) (OtherActor :type Actor%20Object%20Reference) (OtherComp :type Primitive%20Component%20Object%20Reference) (OtherBodyIndex :type Integer) (bFromSweep :type Boolean) (SweepResult :type Hit%20Result%20Structure%20%28by%20ref%29))
  ;[1 0 0.0388 0.3565] Handle overlap
  (if (Class|GameplayStatics|ObjectIsA OtherActor "/Script/Engine.Pawn")
    (bind _asbp_bad_bot_game_mode (Utilities|Casting|CastToBP_BadBotGameMode (Game|GetGameMode)))
    (Default|IncrementScore _asbp_bad_bot_game_mode)
    (CallFunction|WinkOut)))

(event EventTick
  (params (DeltaSeconds :type Float%20%28single-precision%29))
  ;[0 1 0.8068 0.4957] Update Location and Rotation
  (CallFunction|UpdateLocation DeltaSeconds)
  (CallFunction|UpdateRotation DeltaSeconds))

(event EventBeginPlay
  (CallFunction|Winkin)
  (CallFunction|InitializeDeltaRotation)
  ;[0.15 0.02105 0.02736 0.5] Start WinkOut TimeLine
  (Utilities|Time|SetTimerbyEvent (delegate Custom|WinkOut) (Variables|Default|GetLifetime))
  ;[1 0 0.0388 0.3565] Handle overlap
  (Collision|AssignOnComponentBeginOverlap (Variables|Default|GetSphereVolume) (delegate Custom|OnSphereOverlap)))

(fn ConstructionScript)

(fn InitializeDeltaRotation
  (Variables|SphereMovement|SetDelta%20Rotation (* (Math|Random|RandomRotator false) (Variables|SphereMovement|GetRotationScaleFactor))))

(fn UpdateLocation
  (params (Delta%20Seconds :type Float%20%28double-precision%29))
  (Transformation|AddActorWorldOffset (* (Transformation|GetActorForwardVector) (* Delta%20Seconds (Variables|SphereMovement|GetSpeed)))))

(fn UpdateRotation
  (params (Delta%20Seconds :type Float%20%28single-precision%29))
  (Class|Actor|AddActorWorldRotation (* (Variables|SphereMovement|GetDelta%20Rotation) Delta%20Seconds)))

(fn ScaleSphere
  (params (Scale :type Float%20%28single-precision%29))
  (Transformation|SetWorldScale3D (Variables|Default|GetSphereMesh) (Math|Vector|MakeVector Scale Scale Scale)))